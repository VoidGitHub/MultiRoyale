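; BP_Weapon is a gun actor that players pick up through interaction, drop and fire.
; A Dropped/Equipped state switches collision on the mesh and interaction sphere, with physics simulation off in both states and the mesh transform reset on equip.
; Fire spawns a ShotgunProjectile at the Muzzle socket, with velocity aimed at a distant point along the camera's forward vector.
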(event EventBeginPlay
  (CallFunction|SetGunState "NewEnumerator0"))

(event EventOnInteracted
  (params (Player :type Third%20Person%20Character%20Object%20Reference))
  (bind _self self)
  (Default|PickupGun Player _self)
  (CallFunction|SetGunState _self "NewEnumerator1"))

(event EventTick
  (params (DeltaSeconds :type Float%20%28single-precision%29))
  (|CallParentFunction DeltaSeconds) ; This node is disabled and will not be called.\nDrag off pins to build functionality.
)

(event Collision|EventActorBeginOverlap
  (params (OtherActor :type Actor%20Object%20Reference))
  (|CallParentFunction OtherActor) ; This node is disabled and will not be called.\nDrag off pins to build functionality.
)

(fn ConstructionScript
  (|CallParentFunction))

(fn GetInteractionText
  (return "Pick Up"))

(fn GetInteractionTextAttach
  (return (Variables|Default|GetStaticMesh)))

(fn SetGunState
  (params (NewGunState :type EGunState%20Enum :default "NewEnumerator0"))
  (bind _staticmesh (Variables|Default|GetStaticMesh))
  (bind _staticmesh_2 (Variables|Default|GetStaticMesh))
  (bind _output_get (Variables|Default|SetGun%20State NewGunState))
  (switch Utilities|FlowControl|Switch|SwitchonEGunState _output_get
    (:NewEnumerator0
      (Collision|SetCollisionProfileName (Variables|Default|GetSphere) "OverlapAllDynamic" false :!class /Script/Engine.PrimitiveComponent)
      (Physics|SetSimulatePhysics _staticmesh false)
      (Collision|SetCollisionProfileName _staticmesh "DroppedGun" true :!class /Script/Engine.PrimitiveComponent))
    (:NewEnumerator1
      (Collision|SetCollisionProfileName (Variables|Default|GetSphere) "NoCollision" false :!class /Script/Engine.PrimitiveComponent)
      (Physics|SetSimulatePhysics _staticmesh_2 false)
      (Collision|SetCollisionProfileName _staticmesh_2 "NoCollision" true :!class /Script/Engine.PrimitiveComponent)
      (Transformation|ResetRelativeTransform (Variables|Default|GetStaticMesh)))))

(fn DropGun
  (CallFunction|SetGunState "NewEnumerator0"))

(fn Fire
  (params (Player%20Camera :type Camera%20Component%20Object%20Reference))
  (bind _staticmesh (Variables|Default|GetStaticMesh))
  (bind _returnvalue (Transformation|GetSocketLocation _staticmesh "Muzzle"))
  (Game|SpawnActorfromClass "/Game/Weapons/CloseRange/Projectile/ShotgunProjectile.ShotgunProjectile_C" (Math|Transform|MakeTransform _returnvalue "0, 0, 0" "1,1,1") "Undefined" 0 (* (Math|Vector|Normalize (- (+ (Transformation|GetWorldLocation Player%20Camera) (* (Math|Vector|GetForwardVector Player%20Camera) 1e+04)) _returnvalue)) 1e+04) 0))