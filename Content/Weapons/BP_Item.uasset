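; BP_Item is an item actor that shows an interaction prompt while a player is in range.
; OnRange creates the prompt widget for that player's controller and hosts it in a runtime-added, screen-space WidgetComponent with no collision.
; The component snaps to GetInteractionTextAttach (root) and shows text from GetInteractionText ("Interact").
; ExitRange destroys the component, and a validity check prevents duplicate prompts.
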(event EventBeginPlay)

(event EventTick
  (params (DeltaSeconds :type Float%20%28single-precision%29)))

(event EventOnRange
  (params (Player :type Third%20Person%20Character%20Object%20Reference))
  (Variables|Private|GetInteractionWidget
    (:then)
    (:else
      (bind _asplayer_controller (Utilities|Casting|CastToPlayerController (Pawn|GetController Player)))
      (bind _returnvalue (UserInterface|CreateWidget "/Game/Widgets/Weapons/InteractionWidget.InteractionWidget_C" _asplayer_controller (CallFunction|GetInteractionText)))
      (bind _returnvalue_2 (AddComponent|AddWidgetComponent false))
      (bind _output_get (Variables|Private|SetInteractionWidget _returnvalue_2))
      (UserInterface|SetWidget _output_get _returnvalue)
      (Class|WidgetComponent|SetWidgetSpace _output_get "Screen")
      (Class|WidgetComponent|SetDrawatDesiredSize _output_get true)
      (Collision|SetCollisionEnabled _output_get "NoCollision")
      (Transformation|AttachComponentToComponent _output_get (CallFunction|GetInteractionTextAttach) "None" "SnapToTarget" "SnapToTarget" "SnapToTarget" true))))

(event EventExitRange
  (bind _interactionwidget (Variables|Private|GetInteractionWidget)
    (:then
      (Components|DestroyComponent _interactionwidget))
    (:else)))

(fn ConstructionScript)

(fn GetInteractionTextAttach
  (return (Variables|Default|GetDefaultSceneRoot)))

(fn GetInteractionText
  (return "Interact"))